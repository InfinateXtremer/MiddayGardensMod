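; Level utility actor that strips stock spot and point lights from the world when play begins.
; On BeginPlay it gathers all SpotLight actors, then all PointLight actors, and destroys each one lacking the "CustomLight" tag.
; Lights tagged "CustomLight" survive, and the construction script is empty.
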(event `self.ReceiveBeginPlay`
  (bind _outactors (`GameplayStatics.GetAllActorsOfClass` "/Script/Engine.SpotLight"))
  (for _array_element _outactors
    (if (not (`self.ActorHasTag` _array_element "CustomLight"))
      (`self.K2_DestroyActor` _array_element)))
  (bind _outactors_2 (`GameplayStatics.GetAllActorsOfClass` "/Script/Engine.PointLight"))
  (for _array_element_2 _outactors_2
    (if (not (`self.ActorHasTag` _array_element_2 "CustomLight"))
      (`self.K2_DestroyActor` _array_element_2))))

(fn `UserConstructionScript`)
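; BP_PS1Destructible is a breakable prop that shatters when the player charges into it.
; On a static mesh hit by the player character, it checks that character's Ability System Component for the Damage.Charge gameplay tag.
; With the tag present, it reveals the Destructible component, applies damage at the player's location along the hit's normal impulse, and hides the intact static mesh.
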(event `self.StaticMesh.OnComponentHit`
  (params (HitComponent :type "PrimitiveComponent Object Reference") (OtherActor :type "Actor Object Reference") (OtherComp :type "PrimitiveComponent Object Reference") (NormalImpulse :type "Vector Structure") (Hit :type "HitResult Structure (by ref)"))
  (bind _returnvalue (`GameplayStatics.GetPlayerCharacter` 0))
  (bind _destructible (`self.Destructible`))
  (if (== OtherActor _returnvalue)
    (if (`GameplayTagAssetInterface.HasMatchingGameplayTag` (`AbilitySystemBlueprintLibrary.GetAbilitySystemComponent` _returnvalue) (struct :`TagName` "Damage.Charge"))
      (`SceneComponent.SetVisibility` _destructible true false)
      (`DestructibleComponent.ApplyDamage` _destructible 1.0 (`self.K2_GetActorLocation` OtherActor) NormalImpulse 10.0)
      (`SceneComponent.SetVisibility` (`self.StaticMesh`) false false))))

(fn `UserConstructionScript`)
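; BP_RemoveSelectedLights is a one-shot utility actor that switches off a chosen set of lights shortly after play begins.
; After a short delay it casts each ListToRemove entry to Light and hides that light's component, rather than destroying it.
; The actor then destroys itself.
; Its construction script writes the actor's display name to a TextRender component as a label.
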(event `self.ReceiveBeginPlay`
  (`KismetSystemLibrary.Delay` 1.0)
  (for _array_element (`self.ListToRemove`)
    (bind _aslight (cast `Light` (`|ConvertAsset` _array_element)))
    (bind _lightcomponent (`Light.LightComponent` _aslight))
    (`SceneComponent.SetVisibility` _lightcomponent false true)
    (`SceneComponent.SetHiddenInGame` _lightcomponent true true))
  (`self.K2_DestroyActor`))

(fn `UserConstructionScript`
  (`TextRenderComponent.K2_SetText` (`self.TextRender`) (`KismetTextLibrary.Conv_StringToText` (`KismetSystemLibrary.GetDisplayName` self))))
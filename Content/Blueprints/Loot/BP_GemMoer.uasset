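; BP_GemMoer is a loot utility that relocates the level's gems of five colors to stored marker actors at BeginPlay.
; Setting DetectGems makes the construction script add actors tagged with the GemsToDetect enum name to that color's array, then reset the flag like a button.
; MoveGems pairs each color's gem actors with that array by index, only when gems are at least as many as markers.
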(event `self.ReceiveBeginPlay`
  (`self.MoveGems` "NewEnumerator0")
  (`self.MoveGems` "NewEnumerator1")
  (`self.MoveGems` "NewEnumerator2")
  (`self.MoveGems` "NewEnumerator3")
  (`self.MoveGems` "NewEnumerator4"))

(fn `DetectGem`
  (locals (_SelectedGemArray :type "Array of Actor Object Reference"))
  (bind _gemstodetect (`self.GemsToDetect`))
  (bind _returnvalue (`|GetEnumeratorNameAsString` _gemstodetect))
  (if (`self.DetectGems`)
    (`KismetSystemLibrary.PrintString` _returnvalue)
    (bind _outactors (`GameplayStatics.GetAllActorsWithTag` (`KismetStringLibrary.Conv_StringToName` _returnvalue)))
    (for _array_element _outactors
      (`KismetArrayLibrary.Array_AddUnique` (select `/Game/Blueprints/Loot/GemTypes` _gemstodetect :`NewEnumerator0` (`self.S2_Green`) :`NewEnumerator1` (`self.S2_Magenta`) :`NewEnumerator2` (`self.S2_Purple`) :`NewEnumerator3` (`self.S2_Red`) :`NewEnumerator4` (`self.S2_Yellow`)) _array_element))
    (set `self.DetectGems` false)))

(fn `MoveGems`
  (params (ActorClass :type "/Game/Blueprints/Loot/GemTypes Enum" :default "NewEnumerator0"))
  (locals (_SelectedGemArray :type "Array of Actor Object Reference") (_SelectedGemClass :type "Actor Class Reference") (_LevelGemArray :type "Array of Actor Object Reference"))
  (set `local._SelectedGemArray` (select `/Game/Blueprints/Loot/GemTypes` ActorClass :`NewEnumerator0` (`self.S2_Green`) :`NewEnumerator1` (`self.S2_Magenta`) :`NewEnumerator2` (`self.S2_Purple`) :`NewEnumerator3` (`self.S2_Red`) :`NewEnumerator4` (`self.S2_Yellow`)))
  (bind _output_get (set `local._SelectedGemClass` (select `/Game/Blueprints/Loot/GemTypes` ActorClass :`NewEnumerator0` "/GameplayCommon/LevelMechanics/Loot/Loot_Spyro2/BP_S2_Gem_Green.BP_S2_Gem_Green_C" :`NewEnumerator1` "/GameplayCommon/LevelMechanics/Loot/Loot_Spyro2/BP_S2_Gem_Magenta.BP_S2_Gem_Magenta_C" :`NewEnumerator2` "/GameplayCommon/LevelMechanics/Loot/Loot_Spyro2/BP_S2_Gem_Purple.BP_S2_Gem_Purple_C" :`NewEnumerator3` "/GameplayCommon/LevelMechanics/Loot/Loot_Spyro2/BP_S2_Gem_Red.BP_S2_Gem_Red_C" :`NewEnumerator4` "/GameplayCommon/LevelMechanics/Loot/Loot_Spyro2/BP_S2_Gem_Yellow.BP_S2_Gem_Yellow_C" :!type "Actor Class Reference")))
  (bind _outactors (`GameplayStatics.GetAllActorsOfClass` _output_get))
  (set `local._LevelGemArray` _outactors)
  (if (>= (`KismetArrayLibrary.Array_Length` (`local._LevelGemArray`)) (`KismetArrayLibrary.Array_Length` (`local._SelectedGemArray`)))
    (for (_array_element _array_index) (`local._LevelGemArray`)
      (bind _output (`|GetArrayItem` (`local._SelectedGemArray`) _array_index))
      (`/Engine/EditorBlueprintResources/StandardMacros.IsValid` _output
        (:`Is Valid`
          (`self.K2_SetActorLocation` _array_element (`self.K2_GetActorLocation` _output) false false))))))

(fn `UserConstructionScript`
  (`self.DetectGem`))
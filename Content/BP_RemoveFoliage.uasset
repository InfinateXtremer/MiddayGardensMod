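; BP_RemoveFoliage is an actor that clears foliage from a box volume at runtime.
; Three seconds after BeginPlay, it destroys every component overlapping the Box, since both foliage casts and their fallback all end in DestroyComponent, removing whole components rather than single instances.
; It then destroys overlapping InstancedFoliageActors.
; An unconnected branch that would destroy all InstancedFoliageActors in the level never runs.
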(event `self.ReceiveBeginPlay`
  (bind _box (`self.Box`))
  (`KismetSystemLibrary.Delay` 3.0)
  (for _array_element (`PrimitiveComponent.GetOverlappingComponents` _box)
    (bind _asfoliage_instanced_static_mesh_component (cast `FoliageInstancedStaticMeshComponent` _array_element)
      (:`then`
        (`ActorComponent.K2_DestroyComponent` _asfoliage_instanced_static_mesh_component))
      (:`CastFailed`
        (bind _asweeds_foliage_instanced_static_mesh_component (cast `/TfbWEEDS/WEEDS/WEEDS_FoliageInstancedStaticMeshComponent` _array_element)
          (:`then`
            (`ActorComponent.K2_DestroyComponent` _asweeds_foliage_instanced_static_mesh_component))
          (:`CastFailed`
            (`ActorComponent.K2_DestroyComponent` _array_element))))))
  (for _array_element_2 (`PrimitiveComponent.GetOverlappingActors` _box "/Script/Foliage.InstancedFoliageActor")
    (`self.K2_DestroyActor` _array_element_2)))

(fn `UserConstructionScript`)
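; BP_RemoveSelectedActors is a placed helper actor that deletes a chosen list of actors at runtime.
; One second after BeginPlay it resolves each entry in ListToRemove, destroys that actor, then destroys itself.
; Its construction script sets a text render component to the actor's display name, labelling the instance.
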(event `self.ReceiveBeginPlay`
  (`KismetSystemLibrary.Delay` 1.0)
  (for _array_element (`self.ListToRemove`)
    (`self.K2_DestroyActor` (`|ConvertAsset` _array_element)))
  (`self.K2_DestroyActor`))

(fn `UserConstructionScript`
  (`TextRenderComponent.K2_SetText` (`self.TextRender`) (`KismetTextLibrary.Conv_StringToText` (`KismetSystemLibrary.GetDisplayName` self))))